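; Test actor that spawns Rubik's cube cublets when play begins.
; On BeginPlay it copies its Dimension into RubikCubeGameModeBase, then loops from zero to that value, spawning BP_Cublet actors it owns.
; Each cublet is offset from the actor's location by its index times CubletSize, forming a single line rather than a full cube.
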(event `self.ReceiveBeginPlay`
  (bind _asrubik_cube_game_mode_base (cast `RubikCubeGameModeBase` (`GameplayStatics.GetGameMode`)))
  (bind _output_get (set `RubikCubeGameModeBase.Dimension` (`self.Dimension`) _asrubik_cube_game_mode_base))
  (for _index (range (+ _output_get 1))
    (`|SpawnActorFromClass` "/Game/03_Blueprints/BP_Cublet.BP_Cublet_C" (`KismetMathLibrary.MakeTransform` (+ (`self.K2_GetActorLocation`) (* _index (`self.CubletSize`)))) "Undefined" "OverrideRootScale" self null)))

(event `self.ReceiveTick`
  (params (DeltaSeconds :type "Float (single-precision)")))

(fn `UserConstructionScript`)